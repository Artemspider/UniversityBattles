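; BP_Hero is a hero that hands movement and attack-type requests to BP_Director along with its own X/Y coordinates.
; When Test is set, BeginPlay waits briefly, then calls Walk on the director from the hero's position.
; Right mouse cycles through the available abilities with wraparound, sends the selected one to TypeOfAttac and prints it.
; A disconnected test loop of delayed EventLine damage calls remains in the graph.
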(event `self.ReceiveBeginPlay`
  (if (`self.Test`)
    (`KismetSystemLibrary.Delay` 1.0)
    (bind _returnvalue (`GameplayStatics.GetActorOfClass` "/Game/Our_Content/BlueprintAndCpp/BP_Director.BP_Director_C"))
    (bind _asbp_director (cast `/Game/Our_Content/BlueprintAndCpp/BP_Director` _returnvalue))
    (`/Game/Our_Content/BlueprintAndCpp/BP_Director.Walk` _asbp_director (`self.Self_X`) (`self.Self_Y`))))

(event `Key|RightMouseButton`
  (params (Key :type "Key Structure"))
  (bind _output (`|GetArrayItem` (`self.Awaleble_Abilitys`) (`self.Index_Ability`)))
  (:`Pressed`
    (bind _result (`/Engine/EditorBlueprintResources/StandardMacros.IncrementInt` (`self.Index_Ability`))
      (:`  `
        (if (not (< _result (`KismetArrayLibrary.Array_Length` (`self.Awaleble_Abilitys`))))
          (set `self.Index_Ability` 0))
        (bind _returnvalue (`GameplayStatics.GetActorOfClass` "/Game/Our_Content/BlueprintAndCpp/BP_Director.BP_Director_C"))
        (`/Game/Our_Content/BlueprintAndCpp/BP_Director.Type_Of_Attac` _returnvalue _output (`self.Self_X`) (`self.Self_Y`))
        (`KismetSystemLibrary.PrintString` _output)))))

(fn `UserConstructionScript`)