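; BP_OneSquare is a floor tile that generates a grid floor by recursively spawning copies of itself.
; Tiles in the first row spawn neighbors along X up to NHorizontal, and each new one also starts a column along Y up to NVertical.
; Each spawn is offset by StepSpawn from the Cube's location and receives an incremented index.
; A separate Check_position event sphere-traces upward and prints the actor standing on the tile.
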(event `Spawn_Square_Horizontal`
  (bind (_returnvalue_x _returnvalue_y _returnvalue_z) (`KismetMathLibrary.BreakVector` (`SceneComponent.K2_GetComponentLocation` (`self.Cube`))))
  ;[1 1 1] Генерация пола
  (if (== (`self.Y`) 1)
    (if (> (`self.NHorizontal`) (`self.X`))
      (bind _returnvalue (`|SpawnActorFromClass` "BP_OneSquare_C" (`KismetMathLibrary.MakeTransform` (`KismetMathLibrary.MakeVector` (+ _returnvalue_x (`self.StepSpawn`)) _returnvalue_y _returnvalue_z)) "AlwaysSpawn" "MultiplyWithRoot" null null))
      (bind _asbp_one_square (cast `/Game/Our_Content/BlueprintAndCpp/BP_OneSquare` _returnvalue)
        (:`then`
          (bind _result (`/Engine/EditorBlueprintResources/StandardMacros.IncrementInt` (`self.X`))
            (:`  `
              (set `/Game/Our_Content/BlueprintAndCpp/BP_OneSquare.X` _result _asbp_one_square)
              (`self.Spawn_Square_Horizontal` _asbp_one_square)
              (`self.Spawn_Square_Vertical` _asbp_one_square))))
        (:`CastFailed`
          (`KismetSystemLibrary.PrintString` "Fail"))))))

(event `Spawn_Square_Vertical`
  (bind (_returnvalue_x _returnvalue_y _returnvalue_z) (`KismetMathLibrary.BreakVector` (`SceneComponent.K2_GetComponentLocation` (`self.Cube`))))
  ;[1 1 1] Генерация пола
  (if (> (`self.NVertical`) (`self.Y`))
    (bind _returnvalue (`|SpawnActorFromClass` "BP_OneSquare_C" (`KismetMathLibrary.MakeTransform` (`KismetMathLibrary.MakeVector` _returnvalue_x (+ _returnvalue_y (`self.StepSpawn`)) _returnvalue_z)) "AlwaysSpawn" "MultiplyWithRoot" null null))
    (bind _asbp_one_square (cast `/Game/Our_Content/BlueprintAndCpp/BP_OneSquare` _returnvalue)
      (:`then`
        (bind _result (`/Engine/EditorBlueprintResources/StandardMacros.IncrementInt` (`self.Y`))
          (:`  `
            (set `/Game/Our_Content/BlueprintAndCpp/BP_OneSquare.Y` _result _asbp_one_square)
            (`self.Spawn_Square_Vertical` _asbp_one_square))))
      (:`CastFailed`
        (`KismetSystemLibrary.PrintString` "Fail")))))

(event `Check_position`
  (bind _returnvalue (`SceneComponent.K2_GetComponentLocation` (`self.Cube`)))
  ;[1 1 1] чекаем кто где стоит
  (bind _outhit (`KismetSystemLibrary.SphereTraceSingle` :`Start` _returnvalue :`End` (+ _returnvalue (0.0 0.0 100.0)) :`Radius` 10.0 :`TraceChannel` "TraceTypeQuery1" :`DrawDebugType` "ForDuration"))
  (`KismetSystemLibrary.PrintString` (`KismetSystemLibrary.GetDisplayName` (`.HitActor` (`GameplayStatics.BreakHitResult` _outhit)))))

(fn `UserConstructionScript`)