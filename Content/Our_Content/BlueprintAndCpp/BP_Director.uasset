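; BP_Director is an early-stage director Blueprint that currently only debug-prints the contents of an AllXY array.
; After a short delay on BeginPlay, it loops through AllXY and prints the index of each non-empty entry.
; Unconnected nodes would gather all BP_OneSquare actors, store their last index in HowMany and cast each one, but they never run.
; The Call_Directior event and construction script are empty.
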(event `Call_Directior`)

(event `self.ReceiveBeginPlay`
  (`KismetSystemLibrary.Delay` 3.0)
  (for (_array_element _array_index) (`self.AllXY`)
    (if (!= _array_element (`self.None_`))
      (`KismetSystemLibrary.PrintString` (`KismetStringLibrary.Conv_IntToString` _array_index)))))

(fn `UserConstructionScript`)