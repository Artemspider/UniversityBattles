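; BP_Teacher is an AI enemy on a grid that moves and attacks relative to BP_Hero, and whose defeat shows the win screen.
; Time_Walk steps away when the hero is within two cells, otherwise approaches, using helper functions to pick the target cell for BP_Director.
; Time_Attack has BP_Director deal damage scaled by proximity and column alignment.
; Damage updates the health text; a low-health retreat branch is left unconnected.
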(event `Get_Location`
  (bind (_returnvalue_x _returnvalue_y) (`KismetMathLibrary.BreakVector` (`SceneComponent.K2_GetComponentLocation` (`self.Cube`))))
  (set `self.Self_Y` (`KismetMathLibrary.FTrunc` (/ _returnvalue_y 100.0)))
  (set `self.Self_X` (`KismetMathLibrary.FTrunc` (/ _returnvalue_x 100.0))))

(event `self.ReceiveBeginPlay`
  (`self.Get_Location`)
  (if (`self.Test`)
    (`KismetSystemLibrary.Delay` 1.0)
    (bind _returnvalue (`GameplayStatics.GetActorOfClass` "/Game/Our_Content/BlueprintAndCpp/BP_Director.BP_Director_C"))
    (cast `/Game/Our_Content/BlueprintAndCpp/BP_Director` _returnvalue)))

(event `Damage`
  (params (Damage :type "Float (double-precision)") (Type :type String))
  (bind _returnvalue (`GameplayStatics.GetPlayerController` 0))
  ;[1 1 1] Урон
  (`KismetSystemLibrary.PrintString` (`KismetStringLibrary.Conv_DoubleToString` Damage))
  (switch `string` Type
    (:`Default`
      (bind _output_get (set `self.Health` (- (`self.Health`) Damage)))
      (`TextRenderComponent.K2_SetText` (`self.TextRender`) (`KismetTextLibrary.Conv_DoubleToText` _output_get "HalfToEven"))
      (if (<= _output_get 0.0)
        (bind _returnvalue_2 (`|CreateWidget` "/Game/Our_Content/BlueprintAndCpp/UI_Win.UI_Win_C" _returnvalue))
        (`UserWidget.AddToViewport` _returnvalue_2 0)
        (`WidgetBlueprintLibrary.SetInputMode_UIOnlyEx` _returnvalue _returnvalue_2)))))

(event `Time_Walk`
  (bind _self_y (`self.Self_Y`))
  (bind _self_x (`self.Self_X`))
  ;[1 1 1] перемещение
  (bind _returnvalue (`GameplayStatics.GetActorOfClass` "/Game/Our_Content/BlueprintAndCpp/BP_Director.BP_Director_C"))
  (bind _asbp_director (cast `/Game/Our_Content/BlueprintAndCpp/BP_Director` _returnvalue))
  (bind _returnvalue_2 (`GameplayStatics.GetActorOfClass` "/Game/Our_Content/BlueprintAndCpp/BP_Hero.BP_Hero_C"))
  (bind _asbp_hero (cast `/Game/Our_Content/BlueprintAndCpp/BP_Hero` _returnvalue_2))
  (bind _self_x_2 (`/Game/Our_Content/BlueprintAndCpp/BP_Hero.Self_X` _asbp_hero))
  (bind _returnvalue_3 (`KismetMathLibrary.Abs_Int` (- _self_x_2 _self_x)))
  (bind _self_y_2 (`/Game/Our_Content/BlueprintAndCpp/BP_Hero.Self_Y` _asbp_hero))
  (bind _returnvalue_4 (`KismetMathLibrary.Abs_Int` (- _self_y_2 _self_y)))
  (if (<= (+ _returnvalue_3 _returnvalue_4) 2)
    (bind (_fx _fy) (`self.Go Out Hero` (`self.Self_X`) (`self.Self_Y`) _self_x_2 _self_y_2))
    (`/Game/Our_Content/BlueprintAndCpp/BP_Director.Teachers_Walk` _asbp_director _fx _fy)
    (elif (and (> _returnvalue_4 3) (> _returnvalue_3 5))
      (bind (_fx_2 _fy_2) (`self.Go to Hero` _self_x _self_y _self_x_2 _self_y_2 :!label _label))
      (`/Game/Our_Content/BlueprintAndCpp/BP_Director.Teachers_Walk` _asbp_director _fx_2 _fy_2)
      (elif (and (> _returnvalue_3 3) (> _returnvalue_4 5))
        (goto _label)
        (else
          (bind (_fx_3 _fy_3) (`self.Go to Hero_0` (`self.Self_X`) (`self.Self_Y`) _self_x_2 _self_y_2))
          (`/Game/Our_Content/BlueprintAndCpp/BP_Director.Teachers_Walk` _asbp_director _fx_3 _fy_3)))))
  (`self.Get_Location`))

(event `Time_Attack`
  (bind _self_y (`self.Self_Y`))
  (bind _self_x (`self.Self_X`))
  (bind _self_x_2 (`/Game/Our_Content/BlueprintAndCpp/BP_Hero.Self_X` (stale `Time_Walk` _asbp_hero)))
  (bind _self_y_2 (`/Game/Our_Content/BlueprintAndCpp/BP_Hero.Self_Y` (stale `Time_Walk` _asbp_hero)))
  (if (<= (+ (`KismetMathLibrary.Abs_Int` (- _self_x _self_x_2)) (`KismetMathLibrary.Abs_Int` (- _self_y _self_y_2))) 2)
    (`/Game/Our_Content/BlueprintAndCpp/BP_Director.Teachers_Attack` (stale `Time_Walk` _asbp_director) "" 40.0)
    (elif (and (== _self_x_2 _self_x) (<= (`KismetMathLibrary.Abs_Int` (- _self_y _self_y_2)) 5))
      (`/Game/Our_Content/BlueprintAndCpp/BP_Director.Teachers_Attack` (stale `Time_Walk` _asbp_director) "" 30.0)
      (else
        (`/Game/Our_Content/BlueprintAndCpp/BP_Director.Teachers_Attack` (stale `Time_Walk` _asbp_director) "" 5.0)))))

(fn `Go Out Hero`
  (params (X :type Integer) (Y :type Integer) (Hero_X :type Integer) (Hero_Y :type Integer))
  (returns (FX :type Integer) (FY :type Integer))
  (if (and (== X Hero_X) (> Y Hero_Y))
    (if (!= Y 8)
      (return X (+ Y 1))
      (elif (<= X 10)
        (return X (+ X 2))
        (else
          (return (- X 2) Y))))
    (elif (and (< Y Hero_Y) (== X Hero_X))
      (if (!= Y 0)
        (return X (- Y 1))
        (elif (>= X 2)
          (return (- X 2) Y)
          (else
            (return (+ X 2) Y))))
      (elif (and (> X Hero_X) (== Y Hero_Y))
        (if (!= Y 12)
          (return (+ Y 1) X)
          (elif (>= Y 2)
            (return X (- Y 2))
            (else
              (return X (+ Y 2)))))
        (elif (and (< X Hero_X) (== Y Hero_Y))
          (if (!= X 0)
            (return (- X 1) Y)
            (elif (<= Y 6)
              (return X (+ Y 2))
              (else
                (return X (- Y 2)))))
          (elif (and (> Y Hero_Y) (> X Hero_X))
            (return X (+ Y -1))
            (elif (and (< Y Hero_Y) (> X Hero_X))
              (return (- X 1) Y)
              (elif (and (< X Hero_X) (> Y Hero_Y))
                (return (+ X 1) Y)
                (elif (and (< X Hero_X) (< Y Hero_Y))
                  (return X (- Y -1)))))))))))

(fn `Go Out Hero_0`
  (params (X :type Integer) (Y :type Integer) (Hero_X :type Integer) (Hero_Y :type Integer))
  (returns (FX :type Integer) (FY :type Integer))
  (if (and (== X Hero_X) (> Y Hero_Y))
    (if (<= Y 6)
      (return X (+ Y 2))
      (elif (<= X 10)
        (return X (+ X 2))
        (else
          (return (- X 2) Y))))
    (elif (and (< Y Hero_Y) (== X Hero_X))
      (if (>= Y 2)
        (return X (- Y 2))
        (elif (>= X 2)
          (return (- X 2) Y)
          (else
            (return (+ X 2) Y))))
      (elif (and (> X Hero_X) (== Y Hero_Y))
        (if (<= Y 10)
          (return (+ Y 2) X)
          (elif (>= Y 2)
            (return X (- Y 2))
            (else
              (return X (+ Y 2)))))
        (elif (and (< X Hero_X) (== Y Hero_Y))
          (if (>= X 2)
            (return (- X 2) Y)
            (elif (<= Y 6)
              (return X (+ Y 2))
              (else
                (return X (- Y 2)))))
          (elif (and (> Y Hero_Y) (> X Hero_X))
            (return X (+ Y -1))
            (elif (and (< Y Hero_Y) (> X Hero_X))
              (return (- X 1) Y)
              (elif (and (< X Hero_X) (> Y Hero_Y))
                (return (+ X 1) Y)
                (elif (and (< X Hero_X) (< Y Hero_Y))
                  (return X (- Y -1)))))))))))

(fn `Go to Hero`
  (params (X :type Integer) (Y :type Integer) (Hero_X :type Integer) (Hero_Y :type Integer))
  (returns (FX :type Integer) (FY :type Integer))
  (if (and (> Y Hero_Y) (> X Hero_X))
    (return (+ X -1) (+ Y -1))
    (elif (> X Hero_X)
      (return (+ X -2) Y)
      (elif (> Y Hero_Y)
        (return X (+ Hero_Y -2))
        (elif (and (< Y Hero_Y) (< X Hero_X))
          (return (+ X 1) (+ Y 1))
          (elif (< X Hero_X)
            (return (+ X 2) Y)
            (else
              (return X (+ Y 2)))))))))

(fn `Go to Hero_0`
  (params (X :type Integer) (Y :type Integer) (Hero_X :type Integer) (Hero_Y :type Integer))
  (returns (FX :type Integer) (FY :type Integer))
  (if (and (> Y Hero_Y) (> X Hero_X))
    (return (+ X -1) (+ Y -1))
    (elif (> X Hero_X)
      (return (+ X -2) Y)
      (elif (> Y Hero_Y)
        (return X (+ Hero_Y -2))
        (elif (and (< Y Hero_Y) (< X Hero_X))
          (return (+ X 1) (+ Y 1))
          (elif (< X Hero_X)
            (return (+ X 2) Y)
            (else
              (return X (+ Y 2)))))))))

(fn `UserConstructionScript`)